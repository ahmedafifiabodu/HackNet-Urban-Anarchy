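; AI controller for BP_Turrent that runs the BT_Turrent behavior tree and manages which target the turret engages.
; Sight perception adds seen actors to a target list and removes lost ones, clearing the current target if it was lost.
; ControlTurrentSelectedTarget picks a random actor from that list, writes it to both the turret and the "Current Target" blackboard key, and reports whether it found one.
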(event OnTargetPerceptionUpdated(AIPerception)
  (params (Actor :type Actor%20Object%20Reference) (Stimulus :type AI%20Stimulus%20Structure))
  (Variables|Default|SetCurrentActor Actor)
  (bind _returnvalue (Class|AIPerceptionSystem|GetSenseClassforStimulus Stimulus))
  (if (== _returnvalue "/Script/AIModule.AISense_Sight")
    (if (.bSuccessfullySensed (Utilities|Struct|BreakAIStimulus Stimulus))
      (Utilities|Array|AddUnique (Variables|Default|GetAllTargetActors) (Variables|Default|GetCurrentActor))
      (else
        (CallFunction|RemoveTargetActor (Variables|Default|GetCurrentActor))))))

(event EventPossess
  (params (PossessedPawn :type Pawn%20Object%20Reference))
  (bind _asbp_turrent (Utilities|Casting|CastToBP_Turrent PossessedPawn))
  (Variables|Default|SetBP%20Turrent _asbp_turrent)
  (AI|RunBehaviorTree "/Game/Project/Torrent/Behavior/BT_Turrent.BT_Turrent"))

(fn ConstructionScript)

(fn RemoveTargetActor
  (params (TargetActor :type Actor%20Object%20Reference%20%28by%20ref%29))
  (if (== TargetActor (Variables|/Game/Project/Torrent/BP_Turrent.BP_Turrent_C|GetCurrentTarget (Variables|Default|GetBP%20Turrent)))
    (Variables|/Game/Project/Torrent/BP_Turrent.BP_Turrent_C|SetCurrentTarget (Variables|Default|GetBP%20Turrent) 0)
    (AI|Components|Blackboard|ClearValue (Variables|Default|GetBlackboard) (Utilities|Name|MakeLiteralName "Current Target")))
  (Utilities|Array|RemoveItem (Variables|Default|GetAllTargetActors) TargetActor)
  (return))

(fn ChooseTargetActor
  (if (Utilities|Array|IsNotEmpty (Variables|Default|GetAllTargetActors))
    (return (.OutItem (Utilities|Array|Random (Variables|Default|GetAllTargetActors))))
    (else
      (return 0))))

(fn SetTargetActor
  (params (Target%20Actor :type Actor%20Object%20Reference))
  (Variables|/Game/Project/Torrent/BP_Turrent.BP_Turrent_C|SetCurrentTarget (Variables|Default|GetBP%20Turrent) Target%20Actor)
  (AI|Components|Blackboard|SetValueasObject (Variables|Default|GetBlackboard) (Utilities|Name|MakeLiteralName "Current Target") Target%20Actor)
  (return))

(fn ControlTurrentSelectedTarget
  (bind _selectedactor (CallFunction|ChooseTargetActor))
  (Utilities|IsValid _selectedactor
    (:Is%20Valid
      (CallFunction|SetTargetActor _selectedactor)
      (return true))
    (:Is%20Not%20Valid
      (return false))))