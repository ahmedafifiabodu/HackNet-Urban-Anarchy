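; Sentry turret that switches between idle and combat states and fires in bursts at an externally set target.
; State changes update the AI Blackboard and toggle aiming, shield and firing flags along with exposed and targeting-beam effects.
; Tick tracks target position and distance, and fire events spawn a muzzle flash and an actor aimed from an arrow component.
; Delays pace the beam warm-up and the pause after every two shots.
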(event EventBeginPlay
  (Variables|Default|SetBlackboard (AI|GetBlackboard 0)))

(event EventTick
  (params (DeltaSeconds :type Float%20%28single-precision%29))
  (Utilities|IsValid (Variables|Default|GetCurrentTarget)
    (:Is%20Valid
      (bind _currenttarget (Variables|Default|GetCurrentTarget)
        (:then
          (Variables|AnimBP|SetCurrentTargetLocation (+ (Transformation|GetActorLocation _currenttarget) "0.000000,0.000000,40.000000"))
          (Variables|AnimBP|SetCurrentTargetDistance (Transformation|GetDistanceTo _currenttarget self)))
        (:else)))))

(event Custom|Combat%20State
  (Utilities|FlowControl|Delay 1.0)
  (if (not (Variables|AnimBP|GetIsShiledOpen))
    (Variables|AnimBP|SetIsAiming true)
    (Variables|AnimBP|SetIsShiledOpen true)
    (Utilities|IsValid (Variables|Default|GetFX_Expose)
      (:Is%20Valid
        _)
      (:Is%20Not%20Valid
        (bind _returnvalue (Effects|SpawnEmitterAttached "/Game/Project/Torrent/FX/Particles/Turret/P_SentryTurret_Exposed.P_SentryTurret_Exposed" (Variables|Character|GetMesh) "root" "0.000000,0.000000,-20.000000" "0, 0, 0" "0.440000,0.440000,0.440000" "SnapToTarget"))
        (Variables|Default|SetFX_Expose _returnvalue)))
    (Utilities|FlowControl|Delay 1.0)
    (Utilities|IsValid (Variables|Default|GetCurrentTarget)
      (:Is%20Valid
        (Utilities|IsValid (Variables|Default|GetFX_TargettingBeam)
          (:Is%20Valid
            _)
          (:Is%20Not%20Valid
            (bind _returnvalue_2 (Effects|SpawnEmitterAttached "/Game/Project/Torrent/FX/Particles/Turret/P_SentryTurret_TargetingBeam_Idle.P_SentryTurret_TargetingBeam_Idle" (Variables|Character|GetMesh) "TargetingBeam" "0, 0, 0" "0, 0, 0" "1.000000,1.000000,1.000000" "SnapToTarget"))
            (Variables|Default|SetFX_TargettingBeam _returnvalue_2)))
        (Utilities|FlowControl|Delay 1.0)
        (Utilities|IsValid (Variables|Default|GetCurrentTarget)
          (:Is%20Valid
            (Variables|AnimBP|SetIsFiring true))
          (:Is%20Not%20Valid
            _))
        (Utilities|IsValid (Variables|Default|GetFX_TargettingBeam)
          (:Is%20Valid
            (Components|DestroyComponent (Variables|Default|GetFX_TargettingBeam))))))))

(event Custom|Idle%20State
  (Variables|AnimBP|SetIsAiming false)
  (Variables|AnimBP|SetIsShiledOpen false)
  (Variables|AnimBP|SetIsFiring false)
  (Variables|Default|SetBrustCount 0)
  (Utilities|IsValid (Variables|Default|GetFX_Expose)
    (:Is%20Valid
      (Components|DestroyComponent (Variables|Default|GetFX_Expose)))
    (:Is%20Not%20Valid
      _))
  (Utilities|IsValid (Variables|Default|GetFX_TargettingBeam)
    (:Is%20Valid
      (Components|DestroyComponent (Variables|Default|GetFX_TargettingBeam)))))

(event Custom|Turrent%20Fire%20End
  (Utilities|IsValid (Variables|Default|GetCurrentTarget)
    (:Is%20Valid
      (bind _result (Math|Integer|IncrementInt (Variables|Default|GetBrustCount))
        (:%20%20
          (if (== _result 2)
            (Variables|AnimBP|SetIsFiring false)
            (Variables|Default|SetBrustCount 0)
            (Utilities|FlowControl|Delay 2.0)
            (CallFunction|ContFire)))))))

(event Custom|Turrent%20Fire
  (bind _arrow1 (Variables|Default|GetArrow1))
  (bind _returnvalue (Transformation|GetWorldTransform _arrow1))
  (Effects|SpawnEmitterAttached "/Game/Project/Torrent/FX/Particles/Turret/P_SentryTurret_Muzzle_02.P_SentryTurret_Muzzle_02" (Variables|Character|GetMesh) "Muzzle_01" "0, 0, 0" "0, 0, 0" "0.800000,0.800000,0.800000" "SnapToTarget")
  (Transformation|SetWorldRotation (Variables|Default|GetArrow1) (Math|Rotator|FindLookatRotation (Transformation|GetWorldLocation (Variables|Default|GetArrow1)) (Variables|AnimBP|GetCurrentTargetLocation)) false false)
  (Game|SpawnActorfromClass "/Game/Project/Blueprint/BP_Bullets.BP_Bullets_C" (Math|Transform|MakeTransform (.location _returnvalue) (.rotation _returnvalue) "0.500000,0.500000,0.500000") "AlwaysSpawn" "MultiplyWithRoot" 0 0))

(event Custom|Cont%20Fire
  (Utilities|IsValid (Variables|Default|GetCurrentTarget)
    (:Is%20Valid
      (Utilities|IsValid (Variables|Default|GetFX_TargettingBeam)
        (:Is%20Valid
          _)
        (:Is%20Not%20Valid
          (bind _returnvalue (Effects|SpawnEmitterAttached "/Game/Project/Torrent/FX/Particles/Turret/P_SentryTurret_TargetingBeam_Idle.P_SentryTurret_TargetingBeam_Idle" (Variables|Character|GetMesh) "TargetingBeam" "0, 0, 0" "0, 0, 0" "1.000000,1.000000,1.000000" "SnapToTarget"))
          (Variables|Default|SetFX_TargettingBeam _returnvalue)))
      (Utilities|FlowControl|Delay 1.0)
      (Utilities|IsValid (Variables|Default|GetCurrentTarget)
        (:Is%20Valid
          (Variables|AnimBP|SetIsFiring true))
        (:Is%20Not%20Valid
          _))
      (Utilities|IsValid (Variables|Default|GetFX_TargettingBeam)
        (:Is%20Valid
          (Components|DestroyComponent (Variables|Default|GetFX_TargettingBeam)))))))

(event EventCharTurrentSetCombatState
  (params (Combat :type Boolean))
  (switch Utilities|FlowControl|Switch|SwitchonE_TurrentState (Variables|Default|GetTorrentState)
    (:NewEnumerator0
      (if Combat
        (bind _output_get (Variables|Default|SetTorrentState "NewEnumerator1"))
        (AI|Components|Blackboard|SetValueasEnum (Variables|Default|GetBlackboard) (Utilities|Name|MakeLiteralName "TurrentState") _output_get)
        (CallFunction|CombatState)))
    (:NewEnumerator1
      (if (not Combat)
        (bind _output_get_2 (Variables|Default|SetTorrentState "NewEnumerator0"))
        (AI|Components|Blackboard|SetValueasEnum (Variables|Default|GetBlackboard) (Utilities|Name|MakeLiteralName "TurrentState") _output_get_2)
        (CallFunction|IdleState)))))

(fn ConstructionScript)

(fn ControlTurrentSelectedTarget
  (return false))