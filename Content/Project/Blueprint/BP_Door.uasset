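; BP_Door is a double door that the player can open and close by interacting, provided BP_Player has a key.
; A FlipFlop alternately plays and reverses the DoorAnimation timeline, which lerps the yaw of both door meshes to swing them 90 degrees in opposite directions.
; Activate and Deactivate both call ShowArrow, which toggles three arrow components' visibility through another FlipFlop rather than setting an explicit state.
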(event Custom|Show%20Arrow
  (bind _isa (Utilities|FlowControl|FlipFlop)
    (:A
      _)
    (:B
      _))
  (Variables|Default|SetShowArrowVis _isa)
  (Utilities|FlowControl|Sequence
    (:then_0
      (Rendering|SetVisibility (Variables|Default|GetArrow1) (Variables|Default|GetShowArrowVis) false))
    (:then_1
      (Rendering|SetVisibility (Variables|Default|GetArrow2) (Variables|Default|GetShowArrowVis) false))
    (:then_2
      (Rendering|SetVisibility (Variables|Default|GetArrow) (Variables|Default|GetShowArrowVis) false))))

(event EventActivate
  (CallFunction|ShowArrow))

(event EventDeactivate
  (CallFunction|ShowArrow))

(event EventInteract
  (bind _returnvalue (Actor|GetActorOfClass "/Game/Lecture-2-3/Blueprint/BP_Player.BP_Player_C"))
  (if (Variables|/Game/Lecture-2-3/Blueprint/BP_Player.BP_Player_C|GethasKey _returnvalue)
    (Utilities|FlowControl|FlipFlop
      (:A
        (bind _door (Timeline|Door%20Animation Play)
          (:Update
            (Transformation|SetRelativeRotation (Variables|Default|GetDoor%201) (Math|Rotator|MakeRotator 0.0 0.0 (Math|Float|Lerp 1.8e+02 2.7e+02 _door)) false false)
            (Transformation|SetRelativeRotation (Variables|Default|GetDoor%202) (Math|Rotator|MakeRotator 0.0 0.0 (Math|Float|Lerp 0.0 -9e+01 _door)) false false))))
      (:B
        (Timeline|Door%20Animation Reverse)))))

(fn ConstructionScript)