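; BP_Bullets is a projectile actor that damages BP_Robot_Car on contact.
; When its Box overlaps a car that has an AC_OnDamage component, it applies fixed damage through that component.
; It then fires a RadialForce impulse, spawns an impact particle at the car's root, plays a 2D hit sound and destroys itself.
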(event OnComponentBeginOverlap(Box)
  (params (OverlappedComponent :type Primitive%20Component%20Object%20Reference) (OtherActor :type Actor%20Object%20Reference) (OtherComp :type Primitive%20Component%20Object%20Reference) (OtherBodyIndex :type Integer) (bFromSweep :type Boolean) (SweepResult :type Hit%20Result%20Structure%20%28by%20ref%29))
  (bind _asbp_robot_car (Utilities|Casting|CastToBP_Robot_Car OtherActor))
  (Utilities|IsValid (Actor|GetComponentbyClass _asbp_robot_car "/Game/Lecture-4/Damage-System/AC_OnDamage.AC_OnDamage_C")
    (:Is%20Valid
      (Default|TakeDamage (Actor|GetComponentbyClass _asbp_robot_car "/Game/Lecture-4/Damage-System/AC_OnDamage.AC_OnDamage_C") 1e+01)
      (Class|RadialForceComponent|FireImpulse (Variables|Default|GetRadialForce))
      (Effects|SpawnEmitteratLocation "/Game/Project/Torrent/FX/Particles/Turret/P_SentryTurret_Beam_CharacterImpact.P_SentryTurret_Beam_CharacterImpact" (Transformation|GetWorldLocation (Variables|/Script/Engine.Actor|GetRootComponent _asbp_robot_car)))
      (Audio|PlaySound2D "/Game/Project/Torrent/Hit.Hit" 1.0 1.0 0.0 0 0)
      (Actor|DestroyActor))))

(fn ConstructionScript)