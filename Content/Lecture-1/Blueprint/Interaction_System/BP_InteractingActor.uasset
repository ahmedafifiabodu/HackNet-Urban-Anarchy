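; BP_InteractingActor drives an interaction system, detecting and triggering actors through BPI_Interaction_System.
; TickTrace sphere-traces forward from the actor and tracks the hit interactable, sending activate and deactivate messages as focus changes.
; InteractLongRange sends an interact message to that tracked object.
; InteractCloseRange instead sphere-traces in place around the player character, ignoring the player, and messages the hit actor directly.
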(event Custom|TickTrace
  (bind _returnvalue (Transformation|GetActorLocation))
  (bind (_outhit _returnvalue_2) (Collision|SphereTraceByChannel _returnvalue (+ _returnvalue (* (Transformation|GetActorForwardVector) (Variables|Default|GetTrace%20Distance))) 5e+01 "TraceTypeQuery3" false 0 "None"))
  ;[1 1 1] Did It hit?
  (if _returnvalue_2
    ;[1 1 1] Does it Implement Interface?
    (if (Utilities|DoesObjectImplementInterface (.HitActor (Collision|BreakHitResult _outhit)) "/Game/Lecture-1/Blueprint/Interaction_System/BPI_Interaction_System.BPI_Interaction_System_C")
      ;[1 1 1] Current Object == OutHit
      (if (not (== (Variables|Default|GetCurrentActivatableObject) (.HitActor (Collision|BreakHitResult _outhit))))
        (CallFunction|TryDeactiveCurrentActiveInteractive)
        (Class|BPIInteractionSystem|Activate(Message) (.HitActor (Collision|BreakHitResult _outhit)))
        (Variables|Default|SetCurrentActivatableObject (.HitActor (Collision|BreakHitResult _outhit))))
      (else
        (CallFunction|TryDeactiveCurrentActiveInteractive :!label _label)))
    (else
      (goto _label))))

(fn ConstructionScript)

(fn TryDeactiveCurrentActiveInteractive
  (bind _currentactivatableobject (Variables|Default|GetCurrentActivatableObject)
    (:then
      (Class|BPIInteractionSystem|Deactivate(Message) _currentactivatableobject)
      (Variables|Default|SetCurrentActivatableObject 0))
    (:else)))

(fn InteractLongRange
  (bind _currentactivatableobject (Variables|Default|GetCurrentActivatableObject)
    (:then
      (Class|BPIInteractionSystem|Interact(Message) _currentactivatableobject))
    (:else)))

(fn InteractCloseRange
  (bind _returnvalue (Game|GetPlayerCharacter 0))
  (bind _returnvalue_2 (Transformation|GetActorLocation _returnvalue))
  (bind _outhit (Collision|SphereTraceByChannel _returnvalue_2 _returnvalue_2 1e+02 "TraceTypeQuery3" false (Utilities|Array|MakeArray _returnvalue) "None"))
  (Class|BPIInteractionSystem|Interact(Message) (.HitActor (Collision|BreakHitResult _outhit))))