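; BP_Light-1 is an interactable light with a point light and an arrow indicator.
; Interact uses a FlipFlop to alternately hide and show the point light, starting with hiding it.
; Activate and Deactivate show and hide the arrow.
; The construction script applies the LightIntensity variable to the point light, while BeginPlay does nothing and a duplicate intensity call in the event graph is left unconnected.
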(event EventBeginPlay)

(event EventInteract
  (bind _pointlight (Variables|Default|GetPointLight))
  (Utilities|FlowControl|FlipFlop
    (:A
      (Rendering|SetVisibility _pointlight false false))
    (:B
      (Rendering|SetVisibility _pointlight true false))))

(event EventDeactivate
  (Rendering|SetVisibility (Variables|Default|GetArrow) false false))

(event EventActivate
  (Rendering|SetVisibility (Variables|Default|GetArrow) true false))

(fn ConstructionScript
  ;[0.01388 0.03313 1] Setting Light Intensity
  (Rendering|Components|Light|SetIntensity (Variables|Default|GetPointLight) (Variables|Default|GetLight%20Intensity)))