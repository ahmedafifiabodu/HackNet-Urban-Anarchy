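; BP_Light-Switch is an interactable switch that turns a group of lights off and on.
; Interact runs a FlipFlop that alternately hides and shows the LightComponent of each actor in LightActors, starting with hide.
; The FlipFlop assumes the lights start visible, as it never reads their current state.
; Activate and Deactivate show and hide an Arrow component on the switch.
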(event EventDeactivate
  (Rendering|SetVisibility (Variables|Default|GetArrow) false false))

(event EventActivate
  (Rendering|SetVisibility (Variables|Default|GetArrow) true false))

(event EventInteract
  (bind _light_actors (Variables|Default|GetLight%20Actors))
  (Utilities|FlowControl|FlipFlop
    (:A
      (for _array_element _light_actors
        (Rendering|SetVisibility (Actor|GetComponentbyClass _array_element "/Script/Engine.LightComponent") false false)))
    (:B
      (for _array_element_2 _light_actors
        (Rendering|SetVisibility (Actor|GetComponentbyClass _array_element_2 "/Script/Engine.LightComponent") true false)))))

(fn ConstructionScript)