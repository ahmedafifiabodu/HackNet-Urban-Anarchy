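; BP_Area-Effector_Damage is a damage zone that hurts actors carrying an AC_OnDamage component.
; Box collision overlaps add and remove these components from an array, applying damage immediately on both entry and exit.
; A looping timer started on BeginPlay damages every tracked component every two seconds.
; The construction script sets the zone's text render to a custom label.
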(event OnComponentBeginOverlap(BoxCollision)
  (params (OverlappedComponent :type Primitive%20Component%20Object%20Reference) (OtherActor :type Actor%20Object%20Reference) (OtherComp :type Primitive%20Component%20Object%20Reference) (OtherBodyIndex :type Integer) (bFromSweep :type Boolean) (SweepResult :type Hit%20Result%20Structure%20%28by%20ref%29))
  (bind _returnvalue (Actor|GetComponentbyClass OtherActor "/Game/Lecture-4/Damage-System/AC_OnDamage.AC_OnDamage_C"))
  (Utilities|IsValid _returnvalue
    (:Is%20Valid
      (Utilities|Array|Add (Variables|Default|GetArray%20Of%20Damage%20Able%20Component) _returnvalue)
      (Default|TakeDamage _returnvalue (Variables|Default|GetDamage%20Amount)))))

(event OnComponentEndOverlap(BoxCollision)
  (params (OverlappedComponent :type Primitive%20Component%20Object%20Reference) (OtherActor :type Actor%20Object%20Reference) (OtherComp :type Primitive%20Component%20Object%20Reference) (OtherBodyIndex :type Integer))
  (bind _returnvalue (Actor|GetComponentbyClass OtherActor "/Game/Lecture-4/Damage-System/AC_OnDamage.AC_OnDamage_C"))
  (Utilities|IsValid _returnvalue
    (:Is%20Valid
      (Utilities|Array|RemoveItem (Variables|Default|GetArray%20Of%20Damage%20Able%20Component) _returnvalue)
      (Default|TakeDamage _returnvalue (Variables|Default|GetDamage%20Amount)))))

(event Custom|Affect%20Health
  (for _array_element (Variables|Default|GetArray%20Of%20Damage%20Able%20Component)
    (Default|TakeDamage _array_element (Variables|Default|GetDamage%20Amount))))

(event EventBeginPlay
  (Utilities|Time|SetTimerbyEvent (delegate Custom|Affect%20Health) 2.0 true))

(fn ConstructionScript
  (Rendering|Components|TextRender|SetText (Variables|Default|GetTextRender) (Variables|Default|GetCustom%20Text)))