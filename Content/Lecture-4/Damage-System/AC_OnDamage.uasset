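; AC_OnDamage is a health component that handles damage, healing and death notification for its owner.
; BeginPlay stores the starting Health as MaxHealth.
; TakeDamage subtracts within that range while Health is above zero, calls the OnHealthChange dispatcher, and calls OnDeath when Health reaches zero.
; Heal passes a negated amount to TakeDamage, so it shares the clamp and cannot revive at zero health.
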(event EventBeginPlay
  (Variables|Default|SetMax%20Health (Variables|Default|GetHealth)))

(fn TakeDamage
  (params (Damage%20Amount :type Float%20%28double-precision%29))
  (if (> (Variables|Default|GetHealth) 0.0)
    (bind _output_get (Variables|Default|SetHealth (Math|Float|Clamp(Float) (- (Variables|Default|GetHealth) Damage%20Amount) 0.0 (Variables|Default|GetMax%20Health))))
    (Default|CallOnHealthChange (Variables|Default|GetHealth) (Variables|Default|GetMax%20Health))
    (if (<= _output_get 0.0)
      (Default|CallOnDeath))))

(fn Heal
  (params (Heal%20Amount :type Float%20%28double-precision%29))
  (CallFunction|TakeDamage (* Heal%20Amount -1.0)))